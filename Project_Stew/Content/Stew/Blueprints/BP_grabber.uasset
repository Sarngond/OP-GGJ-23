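; BP_grabber is a grappling projectile that returns to its Player and drags other characters it hits along.
; Shortly after spawning, or on a hit, it plays audio or goes straight into the Comeback timeline, halting movement and lerping the sphere to the Player's GrabberSpot.
; Hit tagged third-person characters are lerped there by a second timeline.
; Finishing either timeline, or hitting its own Player, resets the Player and destroys the grabber.
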(event `self.ReceiveBeginPlay`
  (bind _returnvalue (`SceneComponent.K2_GetComponentLocation` (`self.Sphere`)))
  (set `self.Location` _returnvalue)
  (`KismetSystemLibrary.Delay` 0.2)
  (`AudioComponent.Play` (`self.root_return_audio_v1`) 0.0)
  (bind (_direction _newtrack_0) (`Timeline|Comeback` :!label _label)
    (:`Update`
      (set `MovementComponent.Velocity` (0.0 0.0 0.0) (`self.ProjectileMovement`))
      (`SceneComponent.K2_SetWorldLocation` (`self.Sphere`) (`KismetMathLibrary.VLerp` _returnvalue (`SceneComponent.K2_GetComponentLocation` (`/Game/ThirdPerson/Blueprints/BP_ThirdPersonCharacter.grabber_spot` (`self.Player`))) (* _newtrack_0 (`self.grapple speed`))) false false))
    (:`Finished`
      (`/Game/ThirdPerson/Blueprints/BP_ThirdPersonCharacter.Reset` (`self.Player`))
      (`self.K2_DestroyActor`))))

(event `self.Sphere.OnComponentHit`
  (params (HitComponent :type "PrimitiveComponent Object Reference") (OtherActor :type "Actor Object Reference") (OtherComp :type "PrimitiveComponent Object Reference") (NormalImpulse :type "Vector Structure") (Hit :type "HitResult Structure (by ref)"))
  (bind _returnvalue (`KismetSystemLibrary.GetDisplayName` OtherActor))
  (bind _player (`self.Player`))
  (`KismetSystemLibrary.PrintString` _returnvalue)
  (`|ExecutionSequence`
    (:`then_0`
      (goto _label))
    (:`then_1`
      (if (`self.ActorHasTag` OtherActor "Player")
        (if (`KismetStringLibrary.EqualEqual_StrStr` _returnvalue (`KismetSystemLibrary.GetDisplayName` _player))
          (`/Game/ThirdPerson/Blueprints/BP_ThirdPersonCharacter.Reset` _player)
          (`self.K2_DestroyActor`)
          (else
            (bind _asbp_third_person_character (cast `/Game/ThirdPerson/Blueprints/BP_ThirdPersonCharacter` OtherActor))
            (bind (_direction _newtrack_0) (`Timeline|Timeline`)
              (:`Update`
                (`self.K2_SetActorLocation` _asbp_third_person_character (`KismetMathLibrary.VLerp` (`SceneComponent.K2_GetComponentLocation` (`Character.CapsuleComponent` _asbp_third_person_character)) (`SceneComponent.K2_GetComponentLocation` (`/Game/ThirdPerson/Blueprints/BP_ThirdPersonCharacter.grabber_spot` (`self.Player`))) (* _newtrack_0 (`self.grapple speed`))) false false))
              (:`Finished`
                (`/Game/ThirdPerson/Blueprints/BP_ThirdPersonCharacter.Reset` (`self.Player`))
                (`self.K2_DestroyActor`)))))))))

(fn `UserConstructionScript`)