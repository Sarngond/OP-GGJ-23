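; Game instance that tracks player scores and deaths across rounds of a multiplayer last-player-standing game.
; KillPlayer flags a death and recounts the living; when one or none remain, any survivor scores a point.
; CheckWin compares scores to the Goal, then the game opens the end screen on a win or the scoreboard level otherwise.
; UpdateBook passes dead players' roots to CrossOut, which is an empty stub.
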(fn `Check_num_dead`
  (set `self.Players_Alive` (`self.Num_Players`))
  (for _array_element (`self.Is dead`)
    (if _array_element
      (`/Engine/EditorBlueprintResources/StandardMacros.DecrementInt` (`self.Players_Alive`))))
  (`self.Check_Round_Over`))

(fn `Check_Round_Over`
  (if (<= (`self.Players_Alive`) 1)
    (for (_array_element _array_index) (`self.Is dead`)
      (if (not _array_element)
        (`self.Incrment_Player_Score` _array_index)))
    (bind _wining__player (`self.Check_Win`))
    (if (== _wining__player -1)
      (`self.End_Round`)
      (else
        (`self.End_Game`)))))

(fn `Check_Win`
  (returns (`Wining _Player` :type Integer))
  (for (_array_element _array_index) (`self.Scores`)
    (if (>= _array_element (`self.Goal`))
      (set `self.Wining_player` _array_index)))
  (return (`self.Wining_player`)))

(fn `Cross out `
  (params (`Dead root` :type String)))

(fn `End_Game`
  (`GameplayStatics.OpenLevel` (`KismetStringLibrary.Conv_StringToName` "End_Screen")))

(fn `End_Round`
  (`GameplayStatics.OpenLevel` (`KismetStringLibrary.Conv_StringToName` "Score_Borad")))

(fn `Get_Player_Score`
  (params (Player_Index :type Integer))
  (returns (Player_Score :type Integer))
  (return (`|GetArrayItem` (`self.Scores`) Player_Index)))

(fn `Incrment_Player_Score`
  (params (Player_Index :type Integer))
  (`/Engine/EditorBlueprintResources/StandardMacros.IncrementInt` (`|GetArrayItem` (`self.Scores`) (mod Player_Index (`self.Num_Players`)))))

(fn `Kill _Player `
  (params (`Playler Index` :type Integer))
  (bind _is_dead (`self.Is dead`))
  (for (_array_element _array_index) _is_dead
    (`KismetArrayLibrary.Array_Set` _is_dead _array_index (or _array_element (== _array_index `Playler Index`)) true))
  (`self.Check_num_dead`))

(fn `Set Goal`
  (params (Goal :type Integer))
  (set `self.Goal` Goal))

(fn `Update_Book`
  (for (_array_element _array_index) (`self.Is dead`)
    (if _array_element
      (`self.Cross out ` (`|GetArrayItem` (`self.Root`) _array_index)))))