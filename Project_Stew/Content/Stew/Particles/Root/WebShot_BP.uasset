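; WebShot_BP is a web shot effect actor whose Web particle beam follows an assigned projectile.
; Each tick updates the beam's end point and its distance from the Hand component.
; The first player hit disables projectile physics and collision, offsets the beam end toward the hand, sets orientation and fades the Hit parameter via timeline.
; StopEffect drives a Stop timeline, but DestroyRootEffect destroys the effect and actor immediately after calling it.
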(event `StopEffect`
  (`/Engine/EditorBlueprintResources/StandardMacros.DoOnce` false
    (:`Completed`
      (bind (_direction _newtrack) (`Timeline|StopEffect_T`)
        (:`Update`
          (`FXSystemComponent.SetFloatParameter` (`self.Web`) "User.Stop" _newtrack))))))

(event `self.ReceiveBeginPlay`
  (`|ExecutionSequence`))

(event `self.ReceiveTick`
  (params (DeltaSeconds :type "Float (single-precision)"))
  (bind _web (`self.Web`))
  (bind _returnvalue (`SceneComponent.K2_GetComponentLocation` (`Actor.RootComponent` (`self.ProjectileMesh`))))
  (if (not (`self.ProjectileHit`))
    _
    (else
      _))
  (`FXSystemComponent.SetVectorParameter` _web "User.BeamEnd" _returnvalue)
  (`FXSystemComponent.SetFloatParameter` _web "User.Distance" (`KismetMathLibrary.Vector_Distance` _returnvalue (`SceneComponent.K2_GetComponentLocation` (`self.Hand`)))))

(event `Set Projectile`
  (params (`Projectile Mesh` :type "/Game/Stew/Blueprints/BP_grabber Object Reference"))
  (set `self.ProjectileMesh` `Projectile Mesh`))

(event `Destroy Root Effect`
  (`self.StopEffect`)
  (`KismetSystemLibrary.PrintString` "Destroy Root" true true (struct :`R` 1.0 :`G` 0.008451 :`A` 1.0))
  (`ActorComponent.K2_DestroyComponent` (`self.Web`))
  (`self.K2_DestroyActor`))

(event `Hit Player`
  (params (`Hit Result` :type "HitResult Structure"))
  (bind (_bblockinghit _binitialoverlap _time _distance _location _impactpoint) (`GameplayStatics.BreakHitResult` `Hit Result`))
  (bind _web (`self.Web`))
  (bind _sphere (`/Game/Stew/Blueprints/BP_grabber.Sphere` (`self.ProjectileMesh`)))
  (bind _returnvalue (`KismetMathLibrary.Normal` (- _impactpoint (`SceneComponent.K2_GetComponentLocation` (`self.Hand`)))))
  (`/Engine/EditorBlueprintResources/StandardMacros.DoOnce` false
    (:`Completed`
      (set `self.ProjectileHit` true)
      (`PrimitiveComponent.SetSimulatePhysics` _sphere false)
      (`PrimitiveComponent.SetCollisionEnabled` _sphere "NoCollision")
      (`FXSystemComponent.SetVectorParameter` _web "User.BeamEnd" (- _impactpoint (* _returnvalue (`KismetMathLibrary.Conv_DoubleToVector` 40.0))))
      (`FXSystemComponent.SetVectorParameter` _web "User.Orientation" _returnvalue)
      (bind (_direction _hit) (`Timeline|Hit`)
        (:`Update`
          (`FXSystemComponent.SetFloatParameter` (`self.Web`) "User.Hit" _hit))))))

(fn `UserConstructionScript`)